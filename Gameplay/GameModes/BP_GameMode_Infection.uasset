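; Game mode for a round-based Infection match in Squad: survivors on team one against zombies on team two, starting with a random alpha zombie.
; Timers drive waiting for players, pre-round, round limit and post-round steps, updating phase, round wins and notifications on the Infection game state.
; Tick ends the round when no survivors remain and picks a replacement alpha if no zombies are left.
; Between rounds it destroys pawns and the ruleset's queued ragdolls.
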(event Custom|End%20Game
  ;[1 1 1] End Match
  (Default|SetPhase (Variables|Refs|GetGameStateReference) "NewEnumerator4")
  (Class|GameMode|EndMatch))

(event Custom|RoundEnded
  (params (WinningTeam :type ESQTeam%20Enum))
  (bind _postroundtime (Variables|Time|GetPostRoundTime))
  (bind _gamestatereference (Variables|Refs|GetGameStateReference))
  ;[1 1 1] Round End Logic
  (Default|IncRoundsWon _gamestatereference WinningTeam)
  (Default|SetPhase _gamestatereference "NewEnumerator3")
  (if (< (Variables|/Squad_Infection/Gameplay/BP_GameStateV2_Infection.BP_GameStateV2_Infection_C|GetCurrentRound _gamestatereference) (Variables|Config|GetNumberOfRounds))
    (bind _returnvalue (Utilities|Time|SetTimerbyEvent (delegate Custom|RoundInit) _postroundtime))
    (Variables|Time|SetRoundTimer _returnvalue)
    (Default|SendGameNotification (Variables|Refs|GetGameStateReference) "Starting next round" true)
    (else
      (bind _returnvalue_2 (Utilities|Time|SetTimerbyEvent (delegate Custom|End%20Game) _postroundtime))
      (Variables|Time|SetRoundTimer _returnvalue_2))))

(event Custom|Hack%20Player%20Management
  ;[1 1 1] Player Management Hack
)

(event Custom|TimeExpired
  ;[1 1 1] Round End Conditions
  (CallFunction|RoundEnded "Team_One"))

(event Custom|CheckEnoughPlayers
  (bind _gamestatereference (Variables|Refs|GetGameStateReference))
  ;[1 1 1] Wait For Players
  (if (> (Utilities|Set|Length (Variables|/Squad_Infection/Gameplay/BP_GameStateV2_Infection.BP_GameStateV2_Infection_C|GetPlayers (Variables|Refs|GetGameStateReference))) 1)
    (bind _returnvalue (Utilities|Time|SetTimerbyEvent (delegate Custom|StartRound) (Variables|Time|GetPreRoundTime)))
    (Variables|Time|SetRoundTimer _returnvalue)
    (CallFunction|PreparePlayers)
    (Default|SetPhase _gamestatereference "NewEnumerator1")
    (Default|SendGameNotification _gamestatereference "Picking next zombie" true)
    (else
      (Default|SendGameNotification (Variables|Refs|GetGameStateReference) "Waiting for more players" true)
      (Utilities|Time|SetTimerbyEvent (delegate Custom|CheckEnoughPlayers) (Variables|Time|GetPlayerCheckRate)))))

(event Custom|RoundInit
  ;[1 1 1] Round Setup Logic
  (CallFunction|CloseMinimap)
  (CallFunction|CleanupBodies)
  (Default|SetPhase (Variables|Refs|GetGameStateReference) "NewEnumerator5")
  (CallFunction|CheckEnoughPlayers))

(event Custom|NoSurvivorsLeft
  ;[1 1 1] Round End Conditions
  (CallFunction|RoundEnded "Team_Two"))

(event Custom|ZombieLeft
  ;[1 1 1] Find new zombie in match
  (CallFunction|SelectNewZombie)
  (CallFunction|SpawnAlphaZombie)
  (Variables|Default|SetmissingZombie false))

(event Custom|StartRound
  ;[1 1 1] Start Round Logic
  (CallFunction|RoundStartup)
  (bind _returnvalue (Utilities|Time|SetTimerbyEvent (delegate Custom|TimeExpired) (Variables|Time|GetRoundTimeLimit)))
  (Variables|Time|SetRoundTimer _returnvalue)
  (Default|SendGameNotification (Variables|Refs|GetGameStateReference) "" false))

(event EventBeginPlay
  (bind _startuptime (Variables|Default|GetStartupTime))
  (bind _returnvalue (Math|Conversions|ToFloat(Integer) _startuptime))
  ;[1 1 1] Match Setup
  (Variables|Refs|SetGameStateReference (.AsBP%20Game%20State%20V2%20Infection (Utilities|Casting|CastToBP_GameStateV2_Infection (CallFunction|GetSquadGameState))))
  (bind _outactors (Actor|GetAllActorsOfClass "/Squad_Infection/Gameplay/Rulesets/BP_Ruleset_Infection.BP_Ruleset_Infection_C"))
  (Variables|Refs|SetInfectionRulesetReference (Utilities|Array|Get(acopy) _outactors))
  (Default|SetPhase (Variables|Refs|GetGameStateReference) "NewEnumerator0")
  (Default|SetMatchConstants (Variables|Refs|GetGameStateReference) (Variables|Config|GetNumberOfRounds) (Variables|Config|GetVersion) (Variables|Config|GetPlaylist) (Variables|Abilities|GetUAVKills))
  (Default|SetPhase (Variables|Refs|GetGameStateReference) "NewEnumerator5")
  (if (> _returnvalue 0.0)
    (Utilities|Time|SetTimerbyEvent (delegate Custom|CheckEnoughPlayers) _returnvalue)
    (else
      (CallFunction|CheckEnoughPlayers))))

(event EventTick
  (params (DeltaSeconds :type Float%20%28single-precision%29))
  (bind _gamestatereference (Variables|Refs|GetGameStateReference))
  (bind _gamestatereference_2 (Variables|Refs|GetGameStateReference))
  ;[1 1 1] Timer Logic
  (Default|SetTimer _gamestatereference (Variables|Time|GetRoundTimer))
  (if (Utilities|Enum|Equal(Enum) (Variables|/Squad_Infection/Gameplay/BP_GameStateV2_Infection.BP_GameStateV2_Infection_C|GetPhase _gamestatereference) "NewEnumerator2")
    (if (== (Utilities|Set|Length (Variables|/Squad_Infection/Gameplay/BP_GameStateV2_Infection.BP_GameStateV2_Infection_C|GetSurvivors _gamestatereference_2)) 0)
      (CallFunction|NoSurvivorsLeft)
      (elif (and (== 0 (Utilities|Set|Length (Variables|/Squad_Infection/Gameplay/BP_GameStateV2_Infection.BP_GameStateV2_Infection_C|GetZombies _gamestatereference_2))) (not (Variables|Default|GetmissingZombie)))
        (Variables|Default|SetmissingZombie true)
        (CallFunction|ZombieLeft)))))

(event EventPostLogin
  (params (NewPlayer :type Player%20Controller%20Object%20Reference))
  ;[1 1 1] ClientConnection
  (Default|ClientJoined (Variables|Refs|GetGameStateReference) (.AsSQPlayer%20Controller (Utilities|Casting|CastToSQPlayerController NewPlayer))))

(event EventOnSwapPlayerControllers
  (params (OldPC :type Player%20Controller%20Object%20Reference) (NewPC :type Player%20Controller%20Object%20Reference))
  ;[1 1 1] ClientConnection
  (Default|ClientTravel (Variables|Refs|GetGameStateReference) (.AsSQPlayer%20Controller (Utilities|Casting|CastToSQPlayerController OldPC)) (.AsSQPlayer%20Controller (Utilities|Casting|CastToSQPlayerController NewPC))))

(event EventOnLogout
  (params (ExitingController :type Controller%20Object%20Reference))
  ;[1 1 1] ClientConnection
  (Default|ClientLeft (Variables|Refs|GetGameStateReference) (.AsSQPlayer%20Controller (Utilities|Casting|CastToSQPlayerController ExitingController))))

(fn ConstructionScript
  (|CallParentFunction))

(fn PreparePlayers
  (bind _gamestatereference (Variables|Refs|GetGameStateReference))
  (Variables|/Squad_Infection/Gameplay/BP_GameStateV2_Infection.BP_GameStateV2_Infection_C|SetAlphaZombie _gamestatereference 0)
  (Utilities|Set|Clear (Variables|/Squad_Infection/Gameplay/BP_GameStateV2_Infection.BP_GameStateV2_Infection_C|GetSurvivors _gamestatereference))
  (Utilities|Set|Clear (Variables|/Squad_Infection/Gameplay/BP_GameStateV2_Infection.BP_GameStateV2_Infection_C|GetZombies _gamestatereference))
  (bind _result (Utilities|Set|ToArray (Variables|/Squad_Infection/Gameplay/BP_GameStateV2_Infection.BP_GameStateV2_Infection_C|GetPlayers (Variables|Refs|GetGameStateReference))))
  (for _array_element _result
    (if (== (Class|SQPlayerController|GetTeam _array_element) 2)
      (Class|SQGameMode|TrytoChangePlayersTeam _array_element 1 true))
    (Default|AbilityManageEvent (.AsBP%20Player%20Controller%20Infection (Utilities|Casting|CastToBP_PlayerController_Infection _array_element)) true))
  (return))

(fn RoundStartup
  (bind _gamestatereference (Variables|Refs|GetGameStateReference))
  (bind _gamestatereference_2 (Variables|Refs|GetGameStateReference))
  (bind _result (Utilities|Set|Difference (Variables|/Squad_Infection/Gameplay/BP_GameStateV2_Infection.BP_GameStateV2_Infection_C|GetPlayers _gamestatereference) (Variables|/Squad_Infection/Gameplay/BP_GameStateV2_Infection.BP_GameStateV2_Infection_C|GetSurvivors _gamestatereference)))
  (bind _result_2 (Utilities|Set|ToArray _result))
  (bind _output_get (LocalVariables|Set_unspawned _result_2))
  (for _array_element _output_get
    ;[1 1 1] Unspawned
    (CallFunction|SpawnClient _array_element "Team_One")
    (Default|TeamSwitched (.AsBP%20Player%20Controller%20Infection (Utilities|Casting|CastToBP_PlayerController_Infection _array_element))))
  ;[1 1 1] Zombie
  (CallFunction|SelectNewZombie)
  (CallFunction|SpawnAlphaZombie)
  (Default|TeamSwitched (.AsBP%20Player%20Controller%20Infection (Utilities|Casting|CastToBP_PlayerController_Infection (Variables|/Squad_Infection/Gameplay/BP_GameStateV2_Infection.BP_GameStateV2_Infection_C|GetAlphaZombie (Variables|Refs|GetGameStateReference)))))
  (Default|IncCurrentRound _gamestatereference_2)
  (Default|SetPhase _gamestatereference_2 "NewEnumerator2"))

(fn CleanupBodies
  (bind _result (Utilities|Set|ToArray (Variables|/Squad_Infection/Gameplay/BP_GameStateV2_Infection.BP_GameStateV2_Infection_C|GetPlayers (Variables|Refs|GetGameStateReference))))
  (for _array_element (Variables|/Squad_Infection/Gameplay/Rulesets/BP_Ruleset_Infection.BP_Ruleset_Infection_C|GetRagdollQueue (Variables|Refs|GetInfectionRulesetReference))
    (Actor|DestroyActor _array_element))
  (for _array_element_2 _result
    (Actor|DestroyActor (Pawn|GetControlledPawn (.AsSQPlayer%20Controller (Utilities|Casting|CastToSQPlayerController _array_element_2))))))

(fn SpawnAlphaZombie
  (bind _gamestatereference (Variables|Refs|GetGameStateReference))
  (bind _alphazombie (Variables|/Squad_Infection/Gameplay/BP_GameStateV2_Infection.BP_GameStateV2_Infection_C|GetAlphaZombie _gamestatereference))
  (bind _output_get (LocalVariables|Set_isAlive (.bSuccess (Utilities|Casting|CastToSQSoldier (Pawn|GetControlledPawn _alphazombie)))))
  (CallFunction|SpawnClient _alphazombie "Team_Two")
  (if _output_get
    (Default|DisregardDeath (Variables|Refs|GetInfectionRulesetReference) _alphazombie)))

(fn ProcessCleanupQueue
  (bind _cleanupqueue (Variables|GarbageCollection|GetCleanupQueue))
  (LocalVariables|Set_queue (Variables|GarbageCollection|GetCleanupQueue))
  (if (Variables|GarbageCollection|GetBodies)
    (for _array_element (LocalVariables|Get_queue)
      (bind _assqsoldier (Utilities|Casting|CastToSQSoldier _array_element))
      (Utilities|IsValid _assqsoldier
        (:Is%20Valid
          (if (stale _bsuccess)
            (Actor|DestroyActor _assqsoldier)
            (Utilities|Array|RemoveItem _cleanupqueue _assqsoldier))))))
  (if (Variables|GarbageCollection|GetWeapons)
    (for _array_element_2 (LocalVariables|Get_queue)
      (bind _assqweapon (Utilities|Casting|CastToSQWeapon _array_element_2))
      (if (stale _bsuccess)
        (Actor|DestroyActor _assqweapon)
        (Utilities|Array|RemoveItem _cleanupqueue _assqweapon)))
    (Variables|GarbageCollection|SetWeapons false)
    (Variables|GarbageCollection|SetBodies false)))

(fn CloseMinimap
  (bind _outactors (Actor|GetAllActorsOfClass "/Squad_Infection/Blueprints/BP_PlayerController_Infection.BP_PlayerController_Infection_C"))
  (for _array_element _outactors
    (Default|CloseMap _array_element)))

(fn SelectNewZombie
  (bind _survivors (Default|GetSurvivors (Variables|Refs|GetGameStateReference)))
  (bind _result (Utilities|Set|ToArray _survivors))
  (bind _output_get (LocalVariables|Set_zombie (Utilities|Array|Get(acopy) _result (Math|Random|RandomIntegerinRange 0 (Utilities|Array|LastIndex _result)))))
  (Default|SetClientGroup (Variables|Refs|GetGameStateReference) _output_get "Team_Two")
  (bind _output_get_2 (Variables|/Squad_Infection/Gameplay/BP_GameStateV2_Infection.BP_GameStateV2_Infection_C|SetAlphaZombie (Variables|Refs|GetGameStateReference) (LocalVariables|Get_zombie)))
  (Class|SQGameMode|TrytoChangePlayersTeam _output_get_2 2 true))

(fn SpawnClient
  (params (Client :type SQ%20Player%20Controller%20Object%20Reference) (Team :type ESQTeam%20Enum))
  (bind _gamestatereference (Variables|Refs|GetGameStateReference))
  (Default|SetClientGroup _gamestatereference Client Team)
  (switch Utilities|FlowControl|Switch|SwitchonESQTeam Team
    (:Team_One
      (Class|SQPlayerController|SelectSpawn Client (Variables|/Squad_Infection/Gameplay/BP_GameStateV2_Infection.BP_GameStateV2_Infection_C|GetSurvSpawnGroup _gamestatereference)))
    (:Team_Two
      (Class|SQPlayerController|SelectSpawn Client (Variables|/Squad_Infection/Gameplay/BP_GameStateV2_Infection.BP_GameStateV2_Infection_C|GetZomSpawnGroup _gamestatereference))))
  (Class|SQPlayerController|CommitSpawn Client)
  (Class|GameModeBase|RestartPlayer Client))