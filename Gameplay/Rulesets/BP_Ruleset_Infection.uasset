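; Infection mode ruleset that handles deaths, team assignment and respawns by match phase.
; From round start, joiners are forced to team two (zombies), and dead survivors convert, respawning in place via a temporary spawn point; zombies respawn at their spawn group.
; Earlier phases keep everyone except the alpha zombie on team one.
; Round deaths leave a ragdoll made by killing a duplicate pawn; other phases' deaths are uncounted.
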(event Custom|HandleDeath
  (params (Player :type SQ%20Player%20Controller%20Object%20Reference) (Pos :type Transform))
  (bind _gamemodereference (Variables|Default|GetGameModeReference))
  (bind _gamestatereference (Variables|/Squad_Infection/Gameplay/GameModes/BP_GameMode_Infection.BP_GameMode_Infection_C|GetGameStateReference _gamemodereference))
  (bind _phase (Variables|/Squad_Infection/Gameplay/BP_GameStateV2_Infection.BP_GameStateV2_Infection_C|GetPhase _gamestatereference))
  ;[1 1 1] Death Management
  (if (Utilities|Enum|Equal(Enum) _phase "NewEnumerator2")
    (CallFunction|CreateRagdoll Player)
    (else
      (CallFunction|DisregardDeath Player)))
  (switch Utilities|FlowControl|Switch|SwitchonEInfectionPhase _phase
    (:NewEnumerator2
      _)
    (:NewEnumerator3
      _)
    (:NewEnumerator4
      _))
  (if (== (Class|SQPlayerController|GetTeam Player) 1)
    (Default|SetClientGroup _gamestatereference Player "Team_Two")
    (Class|SQGameMode|TrytoChangePlayersTeam (Variables|Default|GetGameModeReference) Player 2 true)
    (CallFunction|RespawninPosition Player Pos)
    (else
      (Utilities|FlowControl|Delay 0.01)
      (CallFunction|RespawnPlayer Player))))

(event Custom|CreateRagdoll
  (params (Player :type SQ%20Player%20Controller%20Object%20Reference))
  ;[1 1 1] Death Management
  (bind _ragdoll (CallFunction|SpawnRagdoll Player))
  (Utilities|FlowControl|Delay 0.1)
  (CallFunction|KillRagdoll _ragdoll)
  (Utilities|Array|AddUnique (Variables|Default|GetRagdollQueue) _ragdoll))

(event EventBeginPlay
  ;[1 1 1] Initialization
  (Variables|Default|SetGameModeReference (.AsBP%20Game%20Mode%20Infection (Utilities|Casting|CastToBP_GameMode_Infection (Game|GetGameMode)))))

(event EventPlayerJoined
  (params (NewPlayer :type SQ%20Player%20Controller%20Object%20Reference)))

(event EventPostPlayerLogout
  (params (Controller :type Controller%20Object%20Reference)))

(event EventPostPlayerLogin
  (params (Controller :type Player%20Controller%20Object%20Reference)))

(event EventPlayerDied
  (params (Victim :type SQ%20Player%20Controller%20Object%20Reference))
  (bind _returnvalue (Pawn|GetControlledPawn Victim))
  ;[1 1 1] Death Management
  (CallFunction|CleanupWeapon _returnvalue)
  (CallFunction|HandleDeath Victim (Transformation|GetActorTransform _returnvalue)))

(event EventPlayerKilled
  (params (Killer :type SQ%20Player%20Controller%20Object%20Reference) (Victim :type SQ%20Player%20Controller%20Object%20Reference))
  ;[1 1 1] Killed Handler
  (Default|AbilityManageEvent (.AsBP%20Player%20Controller%20Infection (Utilities|Casting|CastToBP_PlayerController_Infection Killer)) false)
  (Default|AbilityManageEvent (.AsBP%20Player%20Controller%20Infection (Utilities|Casting|CastToBP_PlayerController_Infection Victim)) true))

(event EventPlayerJoinedTeam
  (params (Player :type SQ%20Player%20Controller%20Object%20Reference) (TeamIndex :type Integer))
  (bind _gamemodereference (Variables|Default|GetGameModeReference))
  (bind _gamemodereference_2 (Variables|Default|GetGameModeReference))
  (bind _gamestatereference (Variables|/Squad_Infection/Gameplay/GameModes/BP_GameMode_Infection.BP_GameMode_Infection_C|GetGameStateReference _gamemodereference))
  ;[1 1 1] Team Management
  (switch Utilities|FlowControl|Switch|SwitchonEInfectionPhase (Variables|/Squad_Infection/Gameplay/BP_GameStateV2_Infection.BP_GameStateV2_Infection_C|GetPhase _gamestatereference)
    (:NewEnumerator0
      (if (and (== TeamIndex 2) (!= Player (Variables|/Squad_Infection/Gameplay/BP_GameStateV2_Infection.BP_GameStateV2_Infection_C|GetAlphaZombie _gamestatereference))) :!label _label
        (Class|SQGameMode|TrytoChangePlayersTeam _gamemodereference_2 Player 1 true)))
    (:NewEnumerator1
      (goto _label))
    (:NewEnumerator5
      (goto _label))
    (:NewEnumerator2
      (if (== TeamIndex 1) :!label _label_2
        (Class|SQGameMode|TrytoChangePlayersTeam _gamemodereference_2 Player 2 true)))
    (:NewEnumerator3
      (goto _label_2))
    (:NewEnumerator4
      (goto _label_2))))

(event EventPlayerSpawned
  (params (NewPlayer :type SQ%20Player%20Controller%20Object%20Reference))
  ;[1 1 1] Spawn Management
  (Default|SetClientGroup (Variables|/Squad_Infection/Gameplay/GameModes/BP_GameMode_Infection.BP_GameMode_Infection_C|GetGameStateReference (Variables|Default|GetGameModeReference)) NewPlayer (Utilities|Enum|ByteToEnumESQTeam (Math|Conversions|ToByte(Integer) (Class|SQPlayerController|GetTeam NewPlayer)))))

(fn ConstructionScript)

(fn DisregardDeath
  (params (Player :type SQ%20Player%20Controller%20Object%20Reference))
  (bind _playerstate (Variables|/Script/Engine.Controller|GetPlayerState Player))
  (bind _assqplayer_state (Utilities|Casting|CastToSQPlayerState _playerstate))
  (Class|SQPlayerState|SetNumDeaths _assqplayer_state (- (Class|SQPlayerState|GetNumDeaths _assqplayer_state) 1)))

(fn SpawnRagdoll
  (params (DeadPlayer :type SQ%20Player%20Controller%20Object%20Reference))
  (bind _returnvalue (Pawn|GetControlledPawn DeadPlayer))
  (bind _returnvalue_2 (Game|SpawnActorfromClass (Utilities|GetClass _returnvalue) (Transformation|GetActorTransform _returnvalue) "AlwaysSpawn" 0 0))
  (Class|SQBlueprintLibrary|SetActorCollisioninGame _returnvalue_2 false true)
  (return (.AsSQSoldier (Utilities|Casting|CastToSQSoldier _returnvalue_2))))

(fn CleanupWeapon
  (params (DeadPlayer :type Pawn%20Object%20Reference))
  (bind _asbp_mutable_soldier (Utilities|Casting|CastToBP_MutableSoldier DeadPlayer))
  (bind _inventorycomponent (Variables|/Script/Squad.SQSoldier|GetInventoryComponent _asbp_mutable_soldier))
  (bind _currentweapon (Variables|/Script/Squad.SQPawnInventoryComponent|GetCurrentWeapon _inventorycomponent))
  (Utilities|IsValid _currentweapon
    (:Is%20Valid
      (Actor|DestroyActor _currentweapon))))

(fn RespawninPosition
  (params (Player :type SQ%20Player%20Controller%20Object%20Reference) (Pos :type Transform))
  (bind _returnvalue (Game|SpawnActorfromClass "/Squad_Infection/Blueprints/SQGameSpawn_Infection.SQGameSpawn_Infection_C" Pos "AlwaysSpawn" 0 0))
  (Class|SQGameSpawn|SetTeam _returnvalue (Utilities|Enum|ByteToEnumESQTeam (Math|Conversions|ToByte(Integer) (Class|SQPlayerController|GetTeam Player))))
  (Class|SQPlayerController|ServerRequestRestartPlayer Player _returnvalue)
  (Actor|DestroyActor _returnvalue)
  (Default|TeamSwitched (.AsBP%20Player%20Controller%20Infection (Utilities|Casting|CastToBP_PlayerController_Infection Player))))

(fn RespawnPlayer
  (params (Player :type SQ%20Player%20Controller%20Object%20Reference))
  (bind _gamemodereference (Variables|Default|GetGameModeReference))
  (bind _gamestatereference (Variables|/Squad_Infection/Gameplay/GameModes/BP_GameMode_Infection.BP_GameMode_Infection_C|GetGameStateReference _gamemodereference))
  (switch Utilities|FlowControl|Switch|SwitchonESQTeam (Utilities|Enum|ByteToEnumESQTeam (Math|Conversions|ToByte(Integer) (Class|SQPlayerController|GetTeam Player)))
    (:Team_One
      (Class|SQPlayerController|ServerRequestRestartPlayer Player (Variables|/Squad_Infection/Gameplay/BP_GameStateV2_Infection.BP_GameStateV2_Infection_C|GetSurvSpawnGroup _gamestatereference)))
    (:Team_Two
      (Class|SQPlayerController|ServerRequestRestartPlayer Player (Variables|/Squad_Infection/Gameplay/BP_GameStateV2_Infection.BP_GameStateV2_Infection_C|GetZomSpawnGroup _gamestatereference)))))

(fn KillRagdoll
  (params (Ragdoll :type Actor%20Object%20Reference))
  (Game|Damage|ApplyDamage Ragdoll 1e+03 0 0)
  (Collision|SetActorEnableCollision Ragdoll false)
  (Utilities|Array|Add (Variables|Default|GetRagdollQueue) Ragdoll))