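; Game state for the Infection mode, tracking players, Survivor (Team One) and Zombie (Team Two) rosters, rounds, timer and match constants.
; Join, leave, travel and team-assignment functions maintain the rosters and counts.
; SetPhase caches team spawn groups in Pre Match, clears the timer Post Round and reports the winner to the Infection ruleset Post Match.
; Winner checks compare constant zeros, always yielding neutral; several functions are stubs.
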(event Custom|SendGameNotification
  (params (Message :type String) (Open :type Boolean))
  (Default|CallGameNotification Message Open))

(event EventBeginPlay
  (Utilities|FlowControl|Delay 5.0)
  (bind _outactors (Actor|GetAllActorsOfClass "/Script/Squad.SQPlayerController"))
  (Utilities|Set|AddItems (Variables|Clients|GetPlayers) _outactors))

(event EventTick
  (params (DeltaSeconds :type Float%20%28single-precision%29)))

(fn ConstructionScript
  (|CallParentFunction))

(fn GetZombies
  (return (Variables|Clients|GetZombies)))

(fn SetClientGroup
  (params (Player :type SQ%20Player%20Controller%20Object%20Reference) (Team :type ESQTeam%20Enum))
  (bind _zombies (Variables|Clients|GetZombies))
  (bind _survivors (Variables|Clients|GetSurvivors))
  (LocalVariables|Set_player Player)
  (switch Utilities|FlowControl|Switch|SwitchonESQTeam Team
    (:Team_One
      (Utilities|Set|Add _survivors (LocalVariables|Get_player))
      (Utilities|Set|Remove _zombies (LocalVariables|Get_player)))
    (:Team_Two
      (Utilities|Set|Add _zombies (LocalVariables|Get_player))
      (Utilities|Set|Remove _survivors (LocalVariables|Get_player))))
  (Variables|Default|SetSurvCount (Utilities|Set|Length _survivors))
  (Variables|Default|SetZomCount (Utilities|Set|Length _zombies))
  (return))

(fn RemoveClient
  (params (Player :type SQ%20Player%20Controller%20Object%20Reference))
  (bind _output_get (LocalVariables|Set_player Player))
  (Utilities|Set|Remove (Variables|Clients|GetSurvivors) _output_get)
  (Utilities|Set|Remove (Variables|Clients|GetZombies) _output_get)
  (Actor|DestroyActor (Variables|/Script/Squad.SQPawnInventoryComponent|GetCurrentWeapon (Variables|/Script/Squad.SQSoldier|GetInventoryComponent (.AsBP%20Mutable%20Soldier (Utilities|Casting|CastToBP_MutableSoldier (Pawn|GetControlledPawn Player))))))
  (Actor|DestroyActor (LocalVariables|Get_player)))

(fn SetAssignment
  (switch Utilities|FlowControl|Switch|SwitchonEInfectionPhase (Variables|Round|GetPhase)))

(fn GetPlayers
  (return (Variables|Clients|GetPlayers)))

(fn SetPhase
  (params (Phase :type EInfectionPhase%20Enum))
  (bind _gamemodereference (Variables|Refs|GetGameModeReference))
  (bind _infectionrulesetreference (Variables|/Squad_Infection/Gameplay/GameModes/BP_GameMode_Infection.BP_GameMode_Infection_C|GetInfectionRulesetReference _gamemodereference))
  (bind _output_get (Variables|Round|SetPhase Phase))
  (switch Utilities|FlowControl|Switch|SwitchonEInfectionPhase _output_get
    (:NewEnumerator0
      (bind _outactors (Actor|GetAllActorsOfClass "/Script/Squad.SQTeamSpawnGroup"))
      (for _array_element _outactors
        (switch Utilities|FlowControl|Switch|SwitchonESQTeam (Class|SQGameSpawn|GetTeam _array_element)
          (:Team_One
            (Variables|Refs|SetSurvSpawnGroup _array_element))
          (:Team_Two
            (Variables|Refs|SetZomSpawnGroup _array_element)))))
    (:NewEnumerator3
      (Utilities|Time|ClearandInvalidateTimerbyHandle (Variables|Round|GetTimerHandle)))
    (:NewEnumerator4
      (if (> 0 0)
        (Class|SQGameModeRuleset|SetWinningTeamfromEnum _infectionrulesetreference "Team_One")
        (elif (> 0 0)
          (Class|SQGameModeRuleset|SetWinningTeamfromEnum _infectionrulesetreference "Team_Two")
          (else
            (Class|SQGameModeRuleset|SetWinningTeamfromEnum _infectionrulesetreference "Team_Neutral")))))))

(fn IncRoundsWon
  (params (Team :type ESQTeam%20Enum))
  (bind _roundswon (Variables|Round|GetRoundsWon))
  (Utilities|Map|Add _roundswon Team (+ (.Value (Utilities|Map|Find _roundswon Team)) 1))
  (return))

(fn GetSurvivors
  (return (Variables|Clients|GetSurvivors)))

(fn IsUAVEnabled
  (params (Team :type ESQTeam%20Enum))
  (return (.Value (Utilities|Map|Find (Variables|Abilities|GetEnableUAV) Team))))

(fn SetMatchConstants
  (params (NumRounds :type Integer) (Version :type String) (Playlist :type EPlaylist%20Enum) (UAVUnlock :type Integer))
  (Variables|Game|SetNumRounds NumRounds)
  (Variables|Game|SetVersion Version)
  (Variables|Game|SetPlaylist Playlist)
  (Utilities|Map|Add (Variables|Abilities|GetAbilities) "NewEnumerator0" UAVUnlock))

(fn SetTimer
  (params (Handle :type Timer%20Handle%20Structure))
  (Variables|Round|SetTimer (Utilities|Time|GetTimerRemainingTimebyHandle Handle)))

(fn IncCurrentRound
  (Math|Integer|IncrementInt (Variables|Round|GetCurrentRound)))

(fn ClientJoined
  (params (Player :type SQ%20Player%20Controller%20Object%20Reference))
  (Utilities|Set|Add (Variables|Clients|GetPlayers) Player))

(fn ClientLeft
  (params (Player :type SQ%20Player%20Controller%20Object%20Reference))
  (Utilities|Set|Remove (Variables|Clients|GetPlayers) Player))

(fn ClientTravel
  (params (OldPlayer :type SQ%20Player%20Controller%20Object%20Reference) (NewPlayer :type SQ%20Player%20Controller%20Object%20Reference))
  (bind _players (Variables|Clients|GetPlayers))
  (Utilities|Set|Remove _players OldPlayer)
  (Utilities|Set|Add _players NewPlayer))

(fn TestState
  (Development|PrintString (Utilities|String|ToString(Integer) (Math|Random|RandomInteger 0))))

(fn NumZombies)

(fn NumSurvivors)