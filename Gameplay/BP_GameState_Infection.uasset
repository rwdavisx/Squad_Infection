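; Game state for the Infection mode, tracking players, their survivor, zombie or unassigned group, the phase and rounds won.
; After a short delay it binds to game mode join, leave and swap events and the ruleset's kill event, whose handler is empty.
; Assignment keeps the three groups mutually exclusive.
; Phase changes stop the round timer post-round and pass the winning team, or neutral on a tie, to the ruleset post-match.
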(event Custom|SendGameNotification
  (params (Message :type String) (Open :type Boolean))
  (Default|CallGameNotification Message Open))

(event Custom|HandlePlayerKilled
  (params (Player :type SQ%20Player%20Controller%20Object%20Reference)))

(event Custom|HandlePlayerJoined
  (params (PlayerController :type SQ%20Player%20Controller%20Object%20Reference))
  (Utilities|Set|Add (Variables|Default|GetPlayers) PlayerController)
  (CallFunction|SetPlayerAssignment 0 "Team_Neutral"))

(event Custom|HandlePlayerLeft
  (params (PlayerController :type SQ%20Player%20Controller%20Object%20Reference))
  (Utilities|Set|Remove (Variables|Default|GetPlayers) PlayerController))

(event Custom|HandlePlayerSwap
  (params (OldPlayerController :type SQ%20Player%20Controller%20Object%20Reference) (NewPlayerController :type SQ%20Player%20Controller%20Object%20Reference))
  (bind _players (Variables|Default|GetPlayers))
  (Utilities|Set|Remove _players OldPlayerController)
  (Utilities|Set|Add _players NewPlayerController))

(event EventBeginPlay
  (bind _gamemodereference (Variables|Default|GetGameModeReference))
  (Utilities|FlowControl|Delay 1.0)
  (EventDispatchers|BindEventtoPlayerJoined _gamemodereference (delegate Custom|HandlePlayerJoined))
  (EventDispatchers|BindEventtoPlayerLeft _gamemodereference (delegate Custom|HandlePlayerLeft))
  (EventDispatchers|BindEventtoPlayerSwap _gamemodereference (delegate Custom|HandlePlayerSwap))
  (EventDispatchers|BindEventtoPlayerKilledEvent (Variables|/Squad_Infection/Gameplay/GameModes/BP_GameMode_Infection.BP_GameMode_Infection_C|GetInfectionRulesetReference _gamemodereference) (delegate Custom|HandlePlayerKilled)))

(event EventTick
  (params (DeltaSeconds :type Float%20%28single-precision%29)))

(fn ConstructionScript
  (|CallParentFunction))

(fn GetNumberOfSurvivors
  (return (Utilities|Array|Length (Variables|Default|GetSurvivors))))

(fn GetNumberOfZombies
  (return (Utilities|Array|Length (Variables|Default|GetZombies))))

(fn GetNumberOfUnassigned
  (return (Utilities|Array|Length (Variables|Default|GetUnassigned))))

(fn SetPlayerAssignment
  (params (Player :type SQ%20Player%20Controller%20Object%20Reference) (Team :type ESQTeam%20Enum))
  (switch Utilities|FlowControl|Switch|SwitchonESQTeam Team
    (:Team_Neutral
      (Utilities|Array|AddUnique (Variables|Default|GetUnassigned) Player)
      (Utilities|Array|RemoveItem (Variables|Default|GetSurvivors) Player)
      (Utilities|Array|RemoveItem (Variables|Default|GetZombies) Player)
      (return))
    (:Team_One
      (Utilities|Array|AddUnique (Variables|Default|GetSurvivors) Player)
      (Utilities|Array|RemoveItem (Variables|Default|GetZombies) Player)
      (Utilities|Array|RemoveItem (Variables|Default|GetUnassigned) Player)
      (return))
    (:Team_Two
      (Utilities|Array|AddUnique (Variables|Default|GetZombies) Player)
      (Utilities|Array|RemoveItem (Variables|Default|GetUnassigned) Player)
      (Utilities|Array|RemoveItem (Variables|Default|GetSurvivors) Player)
      (return))))

(fn UnassignPlayer
  (params (Player :type SQ%20Player%20Controller%20Object%20Reference))
  (Utilities|Array|RemoveItem (Variables|Default|GetSurvivors) Player)
  (Utilities|Array|RemoveItem (Variables|Default|GetZombies) Player)
  (Utilities|Array|RemoveItem (Variables|Default|GetUnassigned) Player)
  (Actor|DestroyActor (Variables|/Script/Squad.SQPawnInventoryComponent|GetCurrentWeapon (Variables|/Script/Squad.SQSoldier|GetInventoryComponent (.AsBP%20Mutable%20Soldier (Utilities|Casting|CastToBP_MutableSoldier (Pawn|GetControlledPawn Player))))))
  (Actor|DestroyActor Player))

(fn SetAssignment
  (switch Utilities|FlowControl|Switch|SwitchonEInfectionPhase (Variables|Default|GetInfectionPhase)))

(fn GetNumberOfPlayers
  (return (Utilities|Set|Length (Variables|Default|GetPlayers))))

(fn SetInfectionPhase
  (params (Phase :type EInfectionPhase%20Enum))
  (bind _survivorsroundswon (Variables|Default|GetSurvivorsRoundsWon))
  (bind _zombiesroundswon (Variables|Default|GetZombiesRoundsWon))
  (bind _gamemodereference (Variables|Default|GetGameModeReference))
  (bind _infectionrulesetreference (Variables|/Squad_Infection/Gameplay/GameModes/BP_GameMode_Infection.BP_GameMode_Infection_C|GetInfectionRulesetReference _gamemodereference))
  (bind _output_get (Variables|Default|SetInfectionPhase Phase))
  (switch Utilities|FlowControl|Switch|SwitchonEInfectionPhase _output_get
    (:NewEnumerator3
      (Utilities|Time|ClearandInvalidateTimerbyHandle (Variables|Default|GetRoundTimer)))
    (:NewEnumerator4
      (if (> _survivorsroundswon _zombiesroundswon)
        (Class|SQGameModeRuleset|SetWinningTeamfromEnum _infectionrulesetreference "Team_One")
        (elif (> _zombiesroundswon _survivorsroundswon)
          (Class|SQGameModeRuleset|SetWinningTeamfromEnum _infectionrulesetreference "Team_Two")
          (else
            (Class|SQGameModeRuleset|SetWinningTeamfromEnum _infectionrulesetreference "Team_Neutral")))))))

(fn SetRoundWinner
  (params (Team :type ESQTeam%20Enum))
  (switch Utilities|FlowControl|Switch|SwitchonESQTeam Team
    (:Team_One
      (Variables|Default|SetSurvivorsRoundsWon (+ (Variables|Default|GetSurvivorsRoundsWon) 1)))
    (:Team_Two
      (Variables|Default|SetZombiesRoundsWon (+ (Variables|Default|GetZombiesRoundsWon) 1)))))