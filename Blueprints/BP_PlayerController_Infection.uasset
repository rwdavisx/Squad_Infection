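; Player controller for the Infection mode, handling killstreak abilities and timed kill and team-switch notifications.
; AbilityManager counts or resets the streak, unlocking a UAV with a standby sound at a game-state threshold.
; F1 spends the UAV, triggering a 15-second team UAV event through the game state unless that team's is already active.
; It also closes the roaming map and cancels spawning on death; airstrike has only a reset flag.
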(event Custom|AbilityManageEvent
  (params (ResetAbilities :type Boolean))
  (CallFunction|AbilityManager ResetAbilities))

(event Custom|TeamSwitched
  (Variables|Default|SetShowTeamNotification true)
  (Utilities|FlowControl|Delay 5.0)
  (Variables|Default|SetShowTeamNotification false))

(event Custom|Close%20Map
  ;[1 1 1] Minimap
  (bind _asbp_hud (Utilities|Casting|CastToBP_HUD (HUD|GetHUD)))
  (Utilities|IsValid (Pawn|GetControlledPawn)
    (:Is%20Valid
      (Default|CloseMenu _asbp_hud false (Variables|/Game/UI/BP_HUD.BP_HUD_C|GetRoamingMap _asbp_hud)))))

(event Custom|KillNotificationEvent
  (params (Notification :type Text))
  (Variables|Default|SetKillNotificationText Notification)
  (Variables|Default|SetShowKillNotification true)
  (Utilities|FlowControl|Delay 5.0)
  (Variables|Default|SetShowKillNotification false))

(event EventBlueprintPlayerDied
  (CallFunction|CancelSpawn))

(event Input|MouseEvents|MouseWheelAxis
  (params (AxisValue :type Float%20%28single-precision%29))
  ;[1 1 1] Minimap
)

(event Input|KeyboardEvents|F1
  (params (Key :type Key%20Structure :default "AnyKey"))
  (bind _returnvalue (Class|SQPlayerController|GetTeam))
  (bind _return_value (CallFunction|GetSquadGameState))
  (bind _returnvalue_2 (Math|Conversions|ToByte(Integer) _returnvalue))
  (bind _asbp_game_state_infection (Utilities|Casting|CastToBP_GameState_Infection _return_value))
  (bind _returnvalue_3 (Utilities|Enum|ByteToEnumESQTeam _returnvalue_2))
  (:Released
    (if (Variables|Default|GetUnlockedUAV)
      (if (not (Variables|Default|GetUsedUAV))
        (Variables|Default|SetUsedUAV true)
        (switch Utilities|FlowControl|Switch|SwitchonESQTeam _returnvalue_3
          (:Team_One
            (if (not (Variables|/Squad_Infection/Gameplay/BP_GameState_Infection.BP_GameState_Infection_C|GetSurvivorsUAV _asbp_game_state_infection))
              (Default|CallUAVEvent _asbp_game_state_infection _returnvalue_3 true :!label _label)
              (switch Utilities|FlowControl|Switch|SwitchonESQTeam _returnvalue_3
                (:Team_One
                  (Variables|/Squad_Infection/Gameplay/BP_GameState_Infection.BP_GameState_Infection_C|SetSurvivorsUAV _asbp_game_state_infection true)
                  (Utilities|FlowControl|Delay 15.0)
                  (Variables|/Squad_Infection/Gameplay/BP_GameState_Infection.BP_GameState_Infection_C|SetSurvivorsUAV _asbp_game_state_infection false))
                (:Team_Two
                  (Variables|/Squad_Infection/Gameplay/BP_GameState_Infection.BP_GameState_Infection_C|SetZombiesUAV _asbp_game_state_infection true)
                  (Utilities|FlowControl|Delay 15.0)
                  (Variables|/Squad_Infection/Gameplay/BP_GameState_Infection.BP_GameState_Infection_C|SetZombiesUAV _asbp_game_state_infection false)))
              (Default|CallUAVEvent _asbp_game_state_infection _returnvalue_3 false)))
          (:Team_Two
            (if (not (Variables|/Squad_Infection/Gameplay/BP_GameState_Infection.BP_GameState_Infection_C|GetZombiesUAV _asbp_game_state_infection))
              (goto _label))))))))

(fn ConstructionScript
  (|CallParentFunction))

(fn IncrementKillstreak
  (Math|Integer|IncrementInt (Variables|Default|GetKillstreak)
    (:%20%20
      (return))))

(fn ResetKillstreak
  (Variables|Default|SetKillstreak 0))

(fn AbilityManager
  (params (ResetAbilities :type Boolean))
  (bind _self self)
  (bind _returnvalue (Pawn|GetControlledPawn _self))
  (bind _asbp_mutable_soldier_infection (Utilities|Casting|CastToBP_MutableSoldier_Infection _returnvalue))
  (bind _gameplayevents (Variables|/Squad_Infection/Blueprints/Soldiers/BP_MutableSoldier_Infection.BP_MutableSoldier_Infection_C|GetGameplayEvents _asbp_mutable_soldier_infection))
  (if ResetAbilities
    (CallFunction|ResetKillstreak)
    (Variables|Default|SetUnlockedUAV false)
    (Variables|Default|SetUnlockedUAV false)
    (Variables|Default|SetUsedUAV false)
    (Variables|Default|SetUsedAirstrike false)
    (else
      (CallFunction|IncrementKillstreak)
      (if (and (not (Variables|Default|GetUnlockedUAV)) (>= (Variables|Default|GetKillstreak) (.Value (Utilities|Map|Find (Variables|/Squad_Infection/Gameplay/BP_GameStateV2_Infection.BP_GameStateV2_Infection_C|GetAbilities (.AsBP%20Game%20State%20V2%20Infection (Utilities|Casting|CastToBP_GameStateV2_Infection (CallFunction|GetSquadGameState)))) "NewEnumerator0"))))
        (Variables|Default|SetUnlockedUAV true)
        (Audio|Components|Audio|SetSound _gameplayevents "/Squad_Infection/Audio/Abilities/UAVStandby.UAVStandby")
        (Audio|Components|Audio|Play _gameplayevents 0.0)
        (elif false
          _)))))