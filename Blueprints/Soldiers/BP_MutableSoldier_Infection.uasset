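; Soldier pawn for the Infection game mode that handles UAV audio alerts and replaces damage with custom rules.
; It plays a sound when its team's UAV activates.
; Point damage hurts only opposing teams during the Round phase, using per-weapon curves sampled by hit time and bone multipliers.
; Radial damage briefly spawns a mapped grenade actor to read its inner radius, then applies massive flat damage to enemy soldiers inside it.
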(event Custom|UAVEvent
  (params (Team :type ESQTeam%20Enum) (IsActive :type Boolean))
  (bind _gameplayevents (Variables|Default|GetGameplayEvents))
  ;[1 1 1] UAV
  (if (== Team (Math|Conversions|ToByte(Integer) (Class|SQSoldier|GetTeam self)))
    (if IsActive
      (Variables|/Script/Engine.AudioComponent|SetSound _gameplayevents "/Squad_Infection/Audio/Abilities/UAVOnline.UAVOnline")
      (Audio|Components|Audio|Play _gameplayevents 0.0))))

(event EventBeginPlay
  ;[1 1 1] Abilities
  (EventDispatchers|BindEventtoUAVActive (.AsBP%20Game%20State%20V2%20Infection (Utilities|Casting|CastToBP_GameStateV2_Infection (CallFunction|GetSquadGameState))) (delegate Custom|UAVEvent)))

(event Game|Damage|EventRadialDamage
  (params (DamageReceived :type Float%20%28single-precision%29) (DamageType :type Damage%20Type%20Object%20Reference) (Origin :type Vector) (HitInfo :type Hit%20Result%20Structure%20%28by%20ref%29) (InstigatedBy :type Controller%20Object%20Reference) (DamageCauser :type Actor%20Object%20Reference))
  ;[1 1 1] Damage Controllers
  (CallFunction|RadialDamageController DamageType Origin HitInfo InstigatedBy DamageCauser))

(event Game|Damage|EventPointDamage
  (params (Damage :type Float%20%28single-precision%29) (DamageType :type Damage%20Type%20Object%20Reference) (HitLocation :type Vector) (HitNormal :type Vector) (HitComponent :type Primitive%20Component%20Object%20Reference) (BoneName :type Name) (ShotFromDirection :type Vector) (InstigatedBy :type Controller%20Object%20Reference) (DamageCauser :type Actor%20Object%20Reference) (HitInfo :type Hit%20Result%20Structure%20%28by%20ref%29))
  ;[1 1 1] Damage Controllers
  (CallFunction|PointDamageController InstigatedBy DamageCauser HitInfo DamageType))

(fn ConstructionScript
  (|CallParentFunction))

(fn PointDamageController
  (params (Instigator :type Controller%20Object%20Reference) (Weapon :type Actor%20Object%20Reference) (HitInfo :type Hit%20Result%20Structure) (DamageType :type Damage%20Type%20Object%20Reference))
  (bind (_bblockinghit _binitialoverlap _time _location _impactpoint _normal _impactnormal _physmat _hitactor _hitcomponent _hitbonename) (Collision|BreakHitResult HitInfo))
  (LocalVariables|Set_damageType (Utilities|GetClass DamageType))
  (LocalVariables|Set_weapon (.AsSQWeapon (Utilities|Casting|CastToSQWeapon Weapon)))
  (bind _output_get (LocalVariables|Set_playerController (.AsSQPlayer%20Controller (Utilities|Casting|CastToSQPlayerController Instigator))))
  (if (!= (Class|SQPlayerController|GetTeam _output_get) (Class|SQSoldier|GetTeam self))
    (switch Utilities|FlowControl|Switch|SwitchonEInfectionPhase (Variables|/Squad_Infection/Gameplay/BP_GameStateV2_Infection.BP_GameStateV2_Infection_C|GetPhase (.AsBP%20Game%20State%20V2%20Infection (Utilities|Casting|CastToBP_GameStateV2_Infection (CallFunction|GetSquadGameState))))
      (:NewEnumerator2
        (Game|Damage|ApplyDamage self (* (Math|Curves|GetFloatValue (.Value (Utilities|Map|Find (LocalVariables|GetWeaponDamageMap) (Utilities|GetClass (LocalVariables|Get_weapon)))) (* (.MaxTime (Math|Curves|GetTimeRange (.Value (Utilities|Map|Find (LocalVariables|GetWeaponDamageMap) (Utilities|GetClass (LocalVariables|Get_weapon)))))) _time)) (.Value (Utilities|Map|Find (LocalVariables|GetBoneDamageMod) _hitbonename))) (LocalVariables|Get_playerController) (LocalVariables|Get_weapon) (LocalVariables|Get_damageType))))))

(fn RadialDamageController
  (params (DamageType :type Damage%20Type%20Object%20Reference) (Origin :type Vector) (HitInfo :type Hit%20Result%20Structure) (InstigatedBy :type Controller%20Object%20Reference) (DamageCauser :type Actor%20Object%20Reference))
  (bind _returnvalue (Game|SpawnActorfromClass (.Value (Utilities|Map|Find (LocalVariables|GetGrenadeDamageMap) (.AsSQGrenade%20Projectile (Utilities|Casting|CastToSQGrenadeProjectileClass (.ProjectileClass (Utilities|Struct|BreakSQGrenadeData (Variables|/Script/Squad.SQGrenade|GetGrenadeConfig (.AsBP%20Generic%20Grenade (Utilities|Casting|CastToBP_GenericGrenade DamageCauser))))))))) (Math|Transform|MakeTransform "0, 0, 0") "Undefined" 0 0))
  (bind _outactors (Collision|SphereOverlapActors Origin (Variables|/Script/Squad.SQProjectile|GetExplosiveDamageInnerRadius _returnvalue) (Utilities|Array|MakeArray "ObjectTypeQuery3") "/Script/Squad.SQSoldier"))
  (for _array_element _outactors
    (if (!= (Class|SQPlayerController|GetTeam (.AsSQPlayer%20Controller (Utilities|Casting|CastToSQPlayerController InstigatedBy))) (Class|SQSoldier|GetTeam (.AsSQSoldier (Utilities|Casting|CastToSQSoldier _array_element))))
      (Game|Damage|ApplyDamage _array_element 1e+04 InstigatedBy DamageCauser (Utilities|GetClass DamageType))))
  (Actor|DestroyActor _returnvalue))