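; Base Blueprint for the M18 smoke grenade item that tints the grenade model with its GrenadeColor.
; The construction script runs the parent's script, then creates dynamic material instances from the first material slot of the first- and third-person meshes.
; It sets the "Top Color" parameter on both instances to GrenadeColor.
; The event graph holds only disabled placeholder events, adding no runtime logic.
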(event EventBeginPlay)

(event Collision|EventActorBeginOverlap
  (params (OtherActor :type Actor%20Object%20Reference)))

(event EventTick
  (params (DeltaSeconds :type Float%20%28single-precision%29))
  (|CallParentFunction 0.0))

(fn ConstructionScript
  (bind _mesh1p (Variables|Default|GetMesh1P))
  (bind _mesh3p (Variables|Default|GetMesh3P))
  (|CallParentFunction)
  (bind _returnvalue (Rendering|Material|CreateDynamicMaterialInstance _mesh1p 0 (Rendering|Material|GetMaterial _mesh1p 0) :!class /Script/Engine.PrimitiveComponent))
  (Rendering|Material|SetVectorParameterValue _returnvalue "Top Color" (Variables|Default|GetGrenadeColor) :!class /Script/Engine.MaterialInstanceDynamic)
  (bind _returnvalue_2 (Rendering|Material|CreateDynamicMaterialInstance _mesh3p 0 (Rendering|Material|GetMaterial _mesh3p 0) :!class /Script/Engine.PrimitiveComponent))
  (Rendering|Material|SetVectorParameterValue _returnvalue_2 "Top Color" (Variables|Default|GetGrenadeColor) :!class /Script/Engine.MaterialInstanceDynamic))