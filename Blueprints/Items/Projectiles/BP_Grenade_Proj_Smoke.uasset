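; Smoke grenade projectile that sets up a delayed, colored smoke cloud effect.
; On BeginPlay it deactivates effects, then, except on dedicated servers, schedules CreateSmoke by name after SmokeDelay.
; It then passes the owning BP_GenericSmokeGrenade's SmokeColor to the SmokeCloud particle system as an instance parameter.
; Tick realigns SmokeCloud to the skeletal mesh rotation with a 90-degree offset, and destruction deactivates effects.
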(event EventBeginPlay
  (Components|Activation|Deactivate)
  (Components|Activation|Deactivate)
  (if (not (Networking|IsDedicatedServer))
    (Utilities|Time|SetTimerbyFunctionName 0 "CreateSmoke" (Variables|Default|GetSmokeDelay))
    (bind _asbp_generic_smoke_grenade (Utilities|Casting|CastToBP_GenericSmokeGrenade (Components|GetOwner)))
    (Utilities|Array|Add (Variables|/Script/Engine.ParticleSystemComponent|GetInstanceParameters (Variables|Default|GetSmokeCloud)) (Utilities|Struct|MakeParticleSysParam "SmokeColorParam" "PSPT_Color" 0.0 0.0 "0, 0, 0" "0, 0, 0" (Math|Conversions|ToColor(LinearColor) (Variables|/Game/Blueprints/Items/Grenades/SmokeGrenades/BP_GenericSmokeGrenade.BP_GenericSmokeGrenade_C|GetSmokeColor _asbp_generic_smoke_grenade))))))

(event EventDestroyed
  (Components|Activation|Deactivate)
  (Components|Activation|Deactivate))

(event EventTick
  (params (DeltaSeconds :type Float%20%28single-precision%29))
  (bind _smokecloud (Variables|Default|GetSmokeCloud))
  (Transformation|SetWorldRotation _smokecloud (.rotation (Transformation|GetWorldTransform (Variables|Default|GetSkeletalMesh))) false false)
  (Transformation|AddRelativeRotation _smokecloud "0, 0,90.000000" false false))

(fn ConstructionScript
  (|CallParentFunction))