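; A 40mm smoke grenade projectile that emits colored smoke and sound when it lands.
; BeginPlay assigns the smoke effect and sound, deactivates both, and feeds the smoke color to the particle system as an instance parameter.
; On non-dedicated-server hits, only a first impact after a minimum flight time triggers CreateSmoke, which starts effect and audio and sleeps the physics body; earlier impacts leave it a dud.
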(event EventDestroyed
  (bind _sound (Variables|Default|GetSound))
  (Components|Activation|Deactivate (Variables|Default|GetEffect))
  (Audio|Components|Audio|Stop _sound)
  (Components|Activation|Deactivate _sound)
  (Utilities|FlowControl|Delay 3.0))

(event EventTick
  (params (DeltaSeconds :type Float%20%28single-precision%29))
  (|CallParentFunction DeltaSeconds))

(event Collision|EventHit
  (params (MyComp :type Primitive%20Component%20Object%20Reference) (Other :type Actor%20Object%20Reference) (OtherComp :type Primitive%20Component%20Object%20Reference) (bSelfMoved :type Boolean) (HitLocation :type Vector :default "0, 0, 0") (HitNormal :type Vector :default "0, 0, 0") (NormalImpulse :type Vector :default "0, 0, 0") (Hit :type Hit%20Result%20Structure%20%28by%20ref%29))
  (if (not (Networking|IsDedicatedServer))
    (if (and (> (Variables|Default|GetFlightTime) (Variables|Default|GetMinFlightTime)) (Variables|Default|GetIsFirstHit))
      (Variables|Default|SetIsFirstHit false)
      (CallFunction|CreateSmoke)
      (else
        (Variables|Default|SetIsFirstHit false)))))

(event EventBeginPlay
  (Audio|Components|Audio|SetSound (Variables|Default|GetSound) (Variables|Default|GetSmokeSound))
  (Effects|Components|ParticleSystem|SetTemplate (Variables|Default|GetEffect) (Variables|Default|GetSmokeEffect))
  (Components|Activation|Deactivate (Variables|Default|GetEffect))
  (Components|Activation|Deactivate (Variables|Default|GetSound))
  (Utilities|Array|Add (Variables|/Script/Engine.ParticleSystemComponent|GetInstanceParameters (Variables|Default|GetEffect)) (Utilities|Struct|MakeParticleSysParam "SmokeColorParam" "PSPT_Color" 0.0 0.0 "0, 0, 0" "0, 0, 0" (Math|Conversions|ToColor(LinearColor) (Variables|Default|GetSmokeColor)))))

(fn ConstructionScript
  (|CallParentFunction))

(fn CreateSmoke
  (bind _sound (Variables|Default|GetSound))
  (Components|Activation|Activate (Variables|Default|GetEffect) false)
  (Components|Activation|Activate _sound false)
  (Audio|Components|Audio|Play _sound 0.0)
  (Class|PrimitiveComponent|PutRigidBodytoSleep (Variables|Default|GetCollisionComp) "None"))