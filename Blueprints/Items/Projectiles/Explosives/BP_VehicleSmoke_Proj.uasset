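; BP_VehicleSmoke_Proj is a vehicle smoke launcher projectile that shows a smoke effect and plays a pop sound.
; On BeginPlay, outside dedicated servers, it assigns the SmokeEffect template to its Effect component, attaches the BTR-80 launcher pop sound to it and activates it.
; Destruction deactivates the effect.
; Both events call the parent first, and the template assignment and deactivation calls are each duplicated.
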(event EventDestroyed
  (|CallParentFunction)
  (Components|Activation|Deactivate (Variables|Default|GetEffect))
  (Components|Activation|Deactivate (Variables|Default|GetEffect)))

(event EventBeginPlay
  (|CallParentFunction)
  (if (not (Networking|IsDedicatedServer))
    (Effects|Components|ParticleSystem|SetTemplate (Variables|Default|GetEffect) (Variables|Default|GetSmokeEffect))
    (Audio|SpawnSoundAttached "/Game/Vehicles/BTR80/Sounds/Smoke/btr80_smokelauncher_pop_Cue.btr80_smokelauncher_pop_Cue" (Variables|Default|GetEffect))
    (Effects|Components|ParticleSystem|SetTemplate (Variables|Default|GetEffect) (Variables|Default|GetSmokeEffect))
    (Components|Activation|Activate (Variables|Default|GetEffect) false)))

(fn ConstructionScript
  (|CallParentFunction))