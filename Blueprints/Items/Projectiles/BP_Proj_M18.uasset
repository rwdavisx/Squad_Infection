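; M18 smoke grenade projectile that tints its mesh to match the smoke color of the grenade that owns it.
; On BeginPlay, outside dedicated servers, it creates a dynamic material on the skeletal mesh and sets Top Color from the owning BP_GenericSmokeGrenade's SmokeColor.
; CreateSmoke puts the rigid body to sleep and activates two components for the smoke effect.
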(event EventBeginPlay
  (bind _skeletalmesh (Variables|Default|GetSkeletalMesh))
  (|CallParentFunction)
  (if (not (Networking|IsDedicatedServer))
    (bind _returnvalue (Rendering|Material|CreateDynamicMaterialInstance _skeletalmesh 0 (Rendering|Material|GetMaterial _skeletalmesh 0) :!class /Script/Engine.PrimitiveComponent))
    (bind _asbp_generic_smoke_grenade (Utilities|Casting|CastToBP_GenericSmokeGrenade (Components|GetOwner)))
    (Rendering|Material|SetVectorParameterValue _returnvalue "Top Color" (Variables|/Game/Blueprints/Items/Grenades/SmokeGrenades/BP_GenericSmokeGrenade.BP_GenericSmokeGrenade_C|GetSmokeColor _asbp_generic_smoke_grenade) :!class /Script/Engine.MaterialInstanceDynamic)))

(fn ConstructionScript
  (|CallParentFunction))

(fn CreateSmoke
  (Class|PrimitiveComponent|PutRigidBodytoSleep "None")
  (Components|Activation|Activate false)
  (Components|Activation|Activate false))