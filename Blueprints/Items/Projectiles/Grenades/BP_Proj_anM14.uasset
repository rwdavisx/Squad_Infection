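; AN-M14 grenade projectile that deals repeated area damage once its fuse expires.
; After the fuse delay, the server starts a looping one-second timer applying radial damage with falloff just above the grenade, while non-server instances call CreateSmoke for the effect.
; The parent BeginPlay call is disabled, and destruction clears the damage timer.
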(event EventBeginPlay
  (if (Networking|IsServer)
    (Utilities|FlowControl|Delay (Variables|Default|GetFuseTime))
    (bind _returnvalue (Utilities|Time|SetTimerbyFunctionName 0 "CauseRadialDamage" 1.0 true))
    (else
      (Utilities|FlowControl|Delay (Variables|Default|GetFuseTime))
      (CallFunction|CreateSmoke))))

(event Collision|EventActorBeginOverlap
  (params (OtherActor :type Actor%20Object%20Reference)))

(event EventTick
  (params (DeltaSeconds :type Float%20%28single-precision%29)))

(event EventDestroyed
  (Utilities|Time|ClearandInvalidateTimerbyHandle (stale EventBeginPlay _returnvalue)))

(fn ConstructionScript
  (|CallParentFunction))

(fn CauseRadialDamage
  (Class|GameplayStatics|ApplyRadialDamagewithFalloff (Variables|Default|GetExplosiveBaseDamage) (Variables|Default|GetExplosiveMinimumDamage) (+ (Transformation|GetActorLocation) "0, 0,20.000000") (Variables|Default|GetExplosiveDamageInnerRadius) (Variables|Default|GetExplosiveDamageOuterRadius) 1.0 (Variables|Default|GetDamageTypeToApply) 0 self (Game|GetInstigatorController) "ECC_Visibility")
  (return))