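; Launched grenade projectile that explodes on its first impact, provided it has flown for a minimum time.
; An earlier first hit permanently disarms that impact trigger.
; BeginPlay attaches an optional lasting-effects actor at the Exhaust socket, which every impact triggers before optional self-destruction.
; Separate events apply direct-hit point damage, noted as needing relocation since projectiles no longer spawn server-side, and spawn explosion particles aligned to the impact normal.
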(event Custom|ServerOnDirectImpact
  (params (HitResult :type Hit%20Result%20Structure) (HitActor :type Actor%20Object%20Reference) (HitFromDirection :type Vector))
  ;[1 1 1] On Direct Impact Damage - projectiles are no longer spawned on the server, so this needs to be done in the player state or player controller
  (Utilities|IsValid HitActor
    (:Is%20Valid
      (if (Variables|/Script/Engine.Actor|GetbCanBeDamaged HitActor)
        (Game|Damage|ApplyPointDamage HitActor (Variables|Default|GetDirect%20Impact%20Damage) HitFromDirection HitResult 0 self (Variables|Default|GetDirect%20Impact%20Damage%20Type))))))

(event EventSpawnEmitter
  (Effects|SpawnEmitteratLocation (Variables|Default|GetExplosionEffect) (Transformation|GetActorLocation) (Math|Rotator|MakeRotfromZ (Variables|Default|GetLastImpactNormal))))

(event EventBeginPlay
  (bind _lastingeffectsactorclass (Variables|Default|GetLastingEffectsActorClass))
  (|CallParentFunction)
  (if (Utilities|IsValidClass _lastingeffectsactorclass)
    (bind _returnvalue (Game|SpawnActorfromClass _lastingeffectsactorclass (Transformation|GetActorTransform) "AlwaysSpawn" 0 0))
    (bind _output_get (Variables|Default|SetLastingEffectsActor _returnvalue))
    (if (Variables|Default|GetbLastingEffectAttachesViaComponentSocket)
      (Transformation|AttachComponentToComponent (VehicleSound|GetRootComponent _output_get) (Variables|Default|GetSkeletalMesh) "Exhaust" "SnapToTarget" "SnapToTarget" "SnapToTarget" true)
      (else
        (Transformation|AttachActorToActor _output_get self "Exhaust" "SnapToTarget" "SnapToTarget" "SnapToTarget" true)))))

(event EventOnImpact
  (params (SelfActor :type Actor%20Object%20Reference) (OtherActor :type Actor%20Object%20Reference) (NormalImpulse :type Vector) (Hit :type Hit%20Result%20Structure%20%28by%20ref%29))
  (bind _lastingeffectsactor (Variables|Default|GetLastingEffectsActor))
  (Variables|Default|SetbHasImpacted true)
  (Variables|Default|SetLastImpactHitResult Hit)
  (if (and (>= (Variables|Default|GetFlightTime) (Variables|Default|GetMinFlightTime)) (Variables|Default|GetIsFirstHit))
    (Variables|Default|SetIsFirstHit false)
    (Variables|Default|SetLastImpactNormal (.Normal (Collision|BreakHitResult Hit)))
    (|CallParentFunction SelfActor OtherActor NormalImpulse Hit)
    (CallFunction|Explode)
    (else
      (Variables|Default|SetIsFirstHit false)))
  (Utilities|IsValid _lastingeffectsactor
    (:Is%20Valid
      (Class|SQLastingEffect|OnTriggerLastingEffectEvent _lastingeffectsactor))
    (:Is%20Not%20Valid
      _))
  (if (Variables|Default|GetbDestroyOnHit)
    (Actor|DestroyActor)))

(event EventTick
  (params (DeltaSeconds :type Float%20%28single-precision%29))
  (|CallParentFunction DeltaSeconds)
  (Variables|Default|SetFlightTime (+ DeltaSeconds (Variables|Default|GetFlightTime))))

(fn ConstructionScript
  (|CallParentFunction))