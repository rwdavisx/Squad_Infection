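; BP_BGM71TOW_Proj is the projectile for the BGM-71 TOW guided missile.
; Its TowDirectionInput event takes a target point and instantly snaps the missile's rotation to face it, using look-at rotation with teleport physics.
; An unconnected RInterpTo chain for turn-rate-limited steering with random flight variation remains in the graph but is unused.
; The construction script only calls its parent.
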(event Custom|TowDirectionInput
  (params (TowDirection :type Vector))
  ;[0 0 0] Targeting
  (Transformation|SetActorRotation (Math|Rotator|FindLookatRotation (Transformation|GetActorLocation) TowDirection) true))

(fn ConstructionScript
  (|CallParentFunction))