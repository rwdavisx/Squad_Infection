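; Kornet guided rocket projectile that follows a tow-style target point while wobbling in flight.
; Each TowDirectionInput event snaps the actor's rotation to look at the supplied target location.
; After the parent BeginPlay, a one-time Timeline adds a sine-driven local Y/Z offset and a constant rotation increment on each update for a corkscrew effect.
; An interpolated turn with random flight variation is left unconnected.
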(event Custom|TowDirectionInput
  (params (TowDirection :type Vector))
  ;[0 0 0] Targeting
  (Transformation|SetActorRotation (Math|Rotator|FindLookatRotation (Transformation|GetActorLocation) TowDirection) true))

(event EventBeginPlay
  ;[1 1 1] Add rotation to projectile
  (Utilities|FlowControl|Sequence
    (:then_0
      (|CallParentFunction))
    (:then_1
      (Utilities|FlowControl|DoOnce false
        (:Completed
          (bind _sine (Timeline|Timeline_0 PlayFromStart)
            (:Update
              (Transformation|AddActorLocalOffset (Math|Vector|MakeVector 0.0 (* _sine 4.0) (* _sine 4.0)) false false)
              (Transformation|AddActorLocalRotation "0, 0,20.000000" false false))))))))

(fn ConstructionScript
  (|CallParentFunction))