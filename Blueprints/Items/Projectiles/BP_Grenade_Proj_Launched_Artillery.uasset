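; Launched artillery grenade projectile that adds incoming-shell audio and destroys itself after a post-impact delay.
; On Tick, where cosmetic events can run (not dedicated servers), it activates descending audio while falling and traces along its velocity for world-static geometry.
; The first trace hit within the trigger distance latches a flag and plays an attached near-ground sound, with optional debug drawing.
; Impact runs parent logic, then waits before destroying the actor.
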(event Custom|OnReachedNearGround
  (Variables|Default|SetbHasReachedNearGround true)
  (Audio|SpawnSoundAttached (Variables|Sound|GetReachedNearGroundSound) (Variables|Default|GetSkeletalMesh) "None" "0, 0, 0" "0, 0, 0" "KeepRelativeOffset" true)
  (if (Variables|Default|GetbDrawDebug)
    (Rendering|Debug|DrawDebugSphere (Transformation|GetActorLocation) 5e+03 12 "(R=1.000000,G=1.000000,B=1.000000,A=1.000000)" 3e+01 2e+01)))

(event EventOnImpact
  (params (SelfActor :type Actor%20Object%20Reference) (OtherActor :type Actor%20Object%20Reference) (NormalImpulse :type Vector) (Hit :type Hit%20Result%20Structure%20%28by%20ref%29))
  (|CallParentFunction SelfActor OtherActor NormalImpulse Hit)
  (Utilities|FlowControl|Delay (Variables|Default|GetLifeTimeAfterImpact))
  (Actor|DestroyActor))

(event EventTick
  (params (DeltaSeconds :type Float%20%28single-precision%29))
  (bind _returnvalue (Transformation|GetActorLocation))
  (|CallParentFunction DeltaSeconds)
  ;[1 1 1] Do not play effects on dedicated servers
  (Networking|CanExecuteCosmeticEvents
    (:True
      ;[1 1 1] Only check if we are descending
      (if (not (Variables|Default|GetbHasReachedNearGround))
        (if (< (.z (Transformation|GetVelocity)) 0.0)
          (Components|Activation|Activate (Variables|Sound|GetDescendingAudio) false)
          (bind (_outhit _returnvalue_2) (Collision|LineTraceForObjects _returnvalue (+ _returnvalue (* (Math|Vector|Normalize (Transformation|GetVelocity)) (Variables|Sound|GetSoundTriggerDistance))) (Utilities|Array|MakeArray "ObjectTypeQuery1") false 0 (select (Variables|Default|GetbDrawDebug) "Persistent" "None") true "(R=1.000000,G=0.000000,B=0.000000,A=1.000000)" "(R=0.000000,G=1.000000,B=0.000000,A=1.000000)" 3e+01))
          (if _returnvalue_2
            (CallFunction|OnReachedNearGround)))))))

(fn ConstructionScript
  (|CallParentFunction))