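; BP_GenericMelee is a generic melee weapon Blueprint that plays first- and third-person soldier swing animations on fire.
; Every fire calls the parent logic, then plays the no-hit montages read from the item's BP_GenericMelee_StaticInfo.
; A valid impact then plays the hit montages, which override the no-hit ones because both share the same montage slot.
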(event EventBeginPlay)

(event Collision|EventActorBeginOverlap
  (params (OtherActor :type Actor%20Object%20Reference)))

(event EventBlueprintonFire
  (params (Origin :type Vector%20%28by%20ref%29))
  ;[1 1 1] Execution order. 1 - Always triggered when firing
  (|CallParentFunction Origin)
  (bind _asbp_generic_melee_static_info (Utilities|Casting|CastToBP_GenericMelee_StaticInfo (Class|SQEquipableItem|GetItemStaticInfo)))
  (Default|CallPlayAnimationEvent 0 (Variables|/Game/Blueprints/Items/Melee/StaticInfo/BP_GenericMelee_StaticInfo.BP_GenericMelee_StaticInfo_C|GetBP_MeleeNoHitSoldier1pMontage _asbp_generic_melee_static_info) (Variables|/Game/Blueprints/Items/Melee/StaticInfo/BP_GenericMelee_StaticInfo.BP_GenericMelee_StaticInfo_C|GetBP_MeleeNoHitSoldier3pMontage _asbp_generic_melee_static_info)))

(event EventTick
  (params (DeltaSeconds :type Float%20%28single-precision%29)))

(event EventPlayImpactEffect
  (params (ImpactHit :type SQ%20Penetration%20Trace%20Structure%20%28by%20ref%29) (bIsProjectileTracer :type Boolean))
  ;[1 1 1] Execution order: 2 - Triggered only if the fire impact is valid - Overrides NoHit montage if triggered (Hit and NoHit are on the same slot)
  (|CallParentFunction ImpactHit bIsProjectileTracer)
  (bind _asbp_generic_melee_static_info (Utilities|Casting|CastToBP_GenericMelee_StaticInfo (Class|SQEquipableItem|GetItemStaticInfo)))
  (Default|CallPlayAnimationEvent 0 (Variables|/Game/Blueprints/Items/Melee/StaticInfo/BP_GenericMelee_StaticInfo.BP_GenericMelee_StaticInfo_C|GetBP_MeleeHitSoldier1pMontage _asbp_generic_melee_static_info) (Variables|/Game/Blueprints/Items/Melee/StaticInfo/BP_GenericMelee_StaticInfo.BP_GenericMelee_StaticInfo_C|GetBP_MeleeHitSoldier3pMontage _asbp_generic_melee_static_info)))

(fn ConstructionScript
  (|CallParentFunction))