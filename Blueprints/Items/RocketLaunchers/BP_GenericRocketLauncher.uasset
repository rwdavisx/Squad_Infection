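; Generic rocket launcher weapon Blueprint that adds backblast when fired.
; On fire, if cosmetic events can execute, it explodes a child-actor shockwave, spawns an emitter, calls SquadBlast's FireBlast and plays a camera shake.
; Shockwave and effects follow the first- or third-person view; construction snaps rear muzzle-flash components to each mesh's backblast socket.
; An unused debug function draws the SquadBlast cone.
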(event EventBeginPlay
  (|CallParentFunction))

(event Collision|EventActorBeginOverlap
  (params (OtherActor :type Actor%20Object%20Reference)))

(event EventBlueprintonFire
  (params (Origin :type Vector%20%28by%20ref%29 :default "0, 0, 0"))
  (bind _returnvalue (Class|SQEquipableItem|IsFirstPersonViewTarget))
  (bind _returnvalue_2 (Class|SQEquipableItem|IsFirstPersonViewTarget))
  (bind _backblastsocket (Variables|Effects|GetBackblastSocket))
  (bind _mesh1p (Variables|Default|GetMesh1P))
  (bind _mesh3p (Variables|Default|GetMesh3P))
  (bind _backblastcomponent1p (Variables|Components|GetBackBlastComponent1P))
  (bind _backblastcomponent3p (Variables|Components|GetBackBlastComponent3P))
  (bind _returnvalue_3 (select _returnvalue _mesh1p _mesh3p))
  (bind _returnvalue_4 (Transformation|GetSocketLocation _returnvalue_3 _backblastsocket))
  (|CallParentFunction Origin)
  (Networking|CanExecuteCosmeticEvents
    (:True
      (bind _asbp_back_blast_shock_wave (Utilities|Casting|CastToBP_BackBlastShockWave (select _returnvalue_2 (Variables|/Script/Engine.ChildActorComponent|GetChildActor _backblastcomponent1p) (Variables|/Script/Engine.ChildActorComponent|GetChildActor _backblastcomponent3p))))
      (Default|Explode _asbp_back_blast_shock_wave (Variables|Default|GetInstigator))
      (Effects|SpawnEmitteratLocation self (select _returnvalue (Variables|Effects|GetBackblastEffect1P) (Variables|Effects|GetBackblastEffect3P)) _returnvalue_4 (select _returnvalue_2 (Transformation|GetWorldRotation _backblastcomponent1p) (Transformation|GetWorldRotation _backblastcomponent3p)))
      (Class|SQBlastComponent|FireBlast (Variables|Components|GetSquadBlast))
      (Camera|PlayWorldCameraShake "/Game/Blueprints/Effects/FireCameraShake_Short.FireCameraShake_Short_C" _returnvalue_4 0.0 1e+02 1.0 true))))

(event EventTick
  (params (DeltaSeconds :type Float%20%28single-precision%29))
  (|CallParentFunction 0.0))

(fn ConstructionScript
  (|CallParentFunction)
  (Variables|/Script/Engine.SceneComponent|SetbAbsoluteScale (Variables|Components|GetMuzzleFlashRearComponent1P) true)
  (Variables|/Script/Engine.SceneComponent|SetbAbsoluteScale (Variables|Components|GetMuzzleFlashRearComponent3P) true)
  (Class|SceneComponent|Attachto (Variables|Components|GetMuzzleFlashRearComponent1P) (Variables|Default|GetMesh1P) (Variables|Effects|GetBackblastSocket) "SnapToTarget" true)
  (Class|SceneComponent|Attachto (Variables|Components|GetMuzzleFlashRearComponent3P) (Variables|Default|GetMesh3P) (Variables|Effects|GetBackblastSocket) "SnapToTarget" true))

(fn DebugDamageVolumeSize
  (bind _squadblast (Variables|Components|GetSquadBlast))
  (bind _returnvalue (Transformation|GetWorldLocation _squadblast))
  (bind _returnvalue_2 (Transformation|GetWorldRotation _squadblast))
  (bind _conelength (Variables|/Script/Squad.SQBlastComponent|GetConeLength _squadblast))
  (bind _coneangle (Variables|/Script/Squad.SQBlastComponent|GetConeAngle _squadblast))
  (bind _returnvalue_3 (Math|Rotator|CombineRotators _returnvalue_2 "-90.000000,0.000000,0.000000"))
  (bind _returnvalue_4 (Math|Rotator|GetRotationXVector _returnvalue_3))
  (Class|KismetSystemLibrary|DrawDebugConeinDegrees (Transformation|GetWorldLocation _squadblast) _returnvalue_4 _conelength _coneangle _coneangle 12 "(R=0.021992,G=1.000000,B=0.137792,A=1.000000)" 0.1 0.0)
  (Rendering|Debug|DrawDebugArrow _returnvalue (+ _returnvalue (* _returnvalue_4 _conelength)) 0.0 "(R=0.895000,G=0.116350,B=0.116350,A=1.000000)" 0.1 0.0)
  (Rendering|Debug|DrawDebugSphere _returnvalue 1e+01 12 "(R=0.050216,G=0.800000,B=0.302574,A=1.000000)" 0.1))